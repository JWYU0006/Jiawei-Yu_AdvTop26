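; BP_GlobalViewer is a camera viewer actor that lets the player orbit a globe with look input.
; On BeginPlay it adds the IMC_Globe Enhanced Input mapping context to player 0 and prints a debug message if a controller is valid.
; The IA_OrbitLook action passes its X and Y values as yaw and pitch to GlobeOrbit's RotateOrbit, which handles the rotation, and prints a debug string.
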(event `self.ReceiveBeginPlay`
  (`EnhancedInputSubsystemInterface.AddMappingContext` (pcsubsystem `EnhancedInputLocalPlayerSubsystem` (`GameplayStatics.GetPlayerController` 0)) "/Game/IMC_Globe.IMC_Globe" 0 (struct))
  ; Comment
  (if (`KismetSystemLibrary.IsValid` (`self.GetController`))
    (`KismetSystemLibrary.PrintString` "possessed")))

(event `EnhancedInput|/Game/IA_OrbitLook`
  (params (ActionValue :type "Vector2D Structure") (ElapsedSeconds :type "Float (double-precision)") (TriggeredSeconds :type "Float (double-precision)") (InputAction :type "InputAction Object Reference" :default "/Game/IA_OrbitLook.IA_OrbitLook"))
  (:`Triggered`
    (`KismetSystemLibrary.PrintString` "Rotating")
    (`GlobeOrbitComponent.RotateOrbit` (`self.GlobeOrbit`) ActionValue_X ActionValue_Y)))

(fn `UserConstructionScript`)